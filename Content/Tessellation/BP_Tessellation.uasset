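; BP_Tessellation builds a procedural mesh with collision at BeginPlay from OBJ-style text in the Teapot data table.
; It parses "v" lines into vertices, printing each, and "f" lines into zero-based indices, ignoring UVs and normals.
; Faces get reversed winding, with quads split into two triangles.
; A cube mesh call is disconnected, and the sine-grid helper functions are not called here.
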(event EventBeginPlay
  (bind _objecttris (Variables|Default|GetobjectTris))
  (bind _objectvertices (Variables|Default|GetobjectVertices))
  (bind _returnvalue (Class|DataTableFunctionLibrary|GetDataTableColumnasString "/Game/teapot.teapot" "Line"))
  (for _array_element _returnvalue
    (if (Utilities|Enum|Equal(Enum) (Utilities|String|GetSubstring _array_element 0 2) "v ")
      (bind _returnvalue_2 (Utilities|Array|Add _objectvertices (Math|Vector|MakeVector (Math|Conversions|ToFloat(Integer) (Utilities|Array|Get(acopy) (Utilities|String|ParseIntoArray _array_element " ") 1)) (Math|Conversions|ToFloat(Integer) (Utilities|Array|Get(acopy) (Utilities|String|ParseIntoArray _array_element " ") 2)) (Math|Conversions|ToFloat(Integer) (Utilities|Array|Get(acopy) (Utilities|String|ParseIntoArray _array_element " ") 3)))))
      (Development|PrintString (Utilities|String|ToString(Vector) (Utilities|Array|Get(acopy) _objectvertices _returnvalue_2)))
      (elif (Utilities|Enum|Equal(Enum) (Utilities|String|GetSubstring _array_element 0 2) "f ")
        (Utilities|Array|Add _objecttris (+ (Math|Conversions|ToInteger(Byte) (Utilities|Array|Get(acopy) (Utilities|String|ParseIntoArray (Utilities|Array|Get(acopy) (Utilities|String|ParseIntoArray _array_element " ") 3) "/"))) -1))
        (Utilities|Array|Add _objecttris (+ (Math|Conversions|ToInteger(Byte) (Utilities|Array|Get(acopy) (Utilities|String|ParseIntoArray (Utilities|Array|Get(acopy) (Utilities|String|ParseIntoArray _array_element " ") 2) "/"))) -1))
        (Utilities|Array|Add _objecttris (+ (Math|Conversions|ToInteger(Byte) (Utilities|Array|Get(acopy) (Utilities|String|ParseIntoArray (Utilities|Array|Get(acopy) (Utilities|String|ParseIntoArray _array_element " ") 1) "/"))) -1))
        (if (not (== (Utilities|Array|Length (Utilities|String|ParseIntoArray _array_element " ")) 4))
          (Utilities|Array|Add _objecttris (+ (Math|Conversions|ToInteger(Byte) (Utilities|Array|Get(acopy) (Utilities|String|ParseIntoArray (Utilities|Array|Get(acopy) (Utilities|String|ParseIntoArray _array_element " ") 1) "/"))) -1))
          (Utilities|Array|Add _objecttris (+ (Math|Conversions|ToInteger(Byte) (Utilities|Array|Get(acopy) (Utilities|String|ParseIntoArray (Utilities|Array|Get(acopy) (Utilities|String|ParseIntoArray _array_element " ") 4) "/"))) -1))
          (Utilities|Array|Add _objecttris (+ (Math|Conversions|ToInteger(Byte) (Utilities|Array|Get(acopy) (Utilities|String|ParseIntoArray (Utilities|Array|Get(acopy) (Utilities|String|ParseIntoArray _array_element " ") 3) "/"))) -1))))))
  (Class|ProceduralMeshComponent|CreateMeshSectionLinearColor (Variables|Default|GetProceduralMesh) 0 (Variables|Default|GetobjectVertices) (Variables|Default|GetobjectTris) 0 0 0 0 0 0 0 true))

(fn ConstructionScript)

(fn CalcSineVertices
  (params (X :type Integer) (Y :type Integer))
  (for _index (range 0 X)
    (for _index_2 (range 0 Y)
      (Utilities|Array|Add (LocalVariables|Getlocal_vertices) (Math|Vector|MakeVector (Math|Conversions|ToFloat(Integer) _index) (Math|Conversions|ToFloat(Integer) _index_2) (Math|Trig|Sin(Radians) (Math|Conversions|ToFloat(Integer) _index_2))))))
  (return (LocalVariables|Getlocal_vertices)))

(fn CalcSineTris
  (params (X :type Integer) (Y :type Integer))
  (bind _local_trisarray (LocalVariables|Getlocal_trisArray))
  (for _index (range 0 X)
    (if (< _index (- X 2))
      (for _index_2 (range 0 Y)
        (if (< (- Y 2) Y)
          (Utilities|Array|Add _local_trisarray _index)
          (Utilities|Array|Add _local_trisarray (+ _index 1))
          (Utilities|Array|Add _local_trisarray (+ _index 6))
          (Utilities|Array|Add _local_trisarray (+ _index 6))
          (Utilities|Array|Add _local_trisarray (+ _index 5))
          (Utilities|Array|Add _local_trisarray _index)))))
  (return (LocalVariables|Getlocal_trisArray)))